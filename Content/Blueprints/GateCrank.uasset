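; GateCrank is a crank actor that drives a Gate, picked by index at BeginPlay, while the player stands in its trigger box.
; Tick uses condition macros and Delays to crank up in steps until open, or back down toward zero once the player leaves.
; Each step rotates the crank, updates CrankValue and messages the Gate.
; E key state is recorded, but its check is disconnected.
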(event `self.ReceiveBeginPlay`
  (bind _outactors (`GameplayStatics.GetAllActorsOfClass` "/Game/Blueprints/Gate.Gate_C"))
  (set `self.ReferencedGate` (`|GetArrayItem` _outactors (`self.GateIndex`))))

(event `Key|E`
  (params (Key :type "Key Structure"))
  ;[1 1 1] Check input
  (:`Pressed`
    (set `self.E pressed ?` true))
  (:`Released`
    (set `self.E pressed ?` false)))

(event `self.ReceiveTick`
  (params (DeltaSeconds :type "Float (single-precision)"))
  ;[1 1 1] Crank up & down
  (if (`self.PlayerOverlapping?`)
    (`self.CheckConditions`
      (:`else`
        (`self.CrankUp`)
        (`self.IsOpen?`)
        (set `self.Open?` true)))
    (else
      (`self.IsClosed?`
        (:`else`
          (`KismetSystemLibrary.Delay` 0.5)
          (`self.CrankDown`)
          (set `self.Open?` false))))))

(event `self.TriggerBox.OnComponentBeginOverlap`
  (params (OverlappedComponent :type "PrimitiveComponent Object Reference") (OtherActor :type "Actor Object Reference") (OtherComp :type "PrimitiveComponent Object Reference") (OtherBodyIndex :type Integer) (bFromSweep :type Boolean) (SweepResult :type "HitResult Structure (by ref)"))
  ;[1 1 1] Check if cranking is possible
  (`self.Overlap player` OtherComp)
  (set `self.PlayerOverlapping?` true))

(event `self.TriggerBox.OnComponentEndOverlap`
  (params (OverlappedComponent :type "PrimitiveComponent Object Reference") (OtherActor :type "Actor Object Reference") (OtherComp :type "PrimitiveComponent Object Reference") (OtherBodyIndex :type Integer))
  ;[1 1 1] Check if cranking is possible
  (`self.Overlap player` OtherComp)
  (if true
    (set `self.PlayerOverlapping?` false)))

(fn `CrankDown`
  (message `/Game/Blueprints/GeneralInterface.UpdateCrank1` (`self.ReferencedGate`) (`self.CrankDownAmount`))
  (`SceneComponent.K2_AddLocalRotation` (`self.Crank`) (struct :`Pitch` -15.0) false false)
  (set `self.CrankValue` (+ (`self.CrankValue`) (`self.CrankDownAmount`))))

(fn `CrankUp`
  (message `/Game/Blueprints/GeneralInterface.UpdateCrank1` (`self.ReferencedGate`) (`self.CrankUpAmount`))
  (`SceneComponent.K2_AddLocalRotation` (`self.Crank`) (struct :`Pitch` 30.0) false false)
  (set `self.CrankValue` (+ (`self.CrankValue`) (`self.CrankUpAmount`))))

(fn `Is open?`
  (returns (ReturnValue :type Boolean))
  (return (or (== (`self.CrankValue`) (`self.OpenValue`)) (== (`self.CrankValue`) (+ (`self.OpenValue`) (`self.CrankDownAmount`))))))

(fn `UserConstructionScript`)