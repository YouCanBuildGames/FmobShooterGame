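; AmbientSoundCue is an actor that switches on its FMOD ambient sound in response to a level trigger.
; On BeginPlay a boolean chooses the source: a TriggerBox's player-detected event or a GateCrank's gate-opened event.
; The source actor is picked by index from a GetAllActorsOfClass result, and either event activates the FmodEvent component without a reset.
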(event `self.ReceiveBeginPlay`
  (if (`self.Trigger by Box (true) Crank (false)`)
    (bind _outactors (`GameplayStatics.GetAllActorsOfClass` "/Game/Blueprints/TriggerBox.TriggerBox_C"))
    (add `/Game/Blueprints/TriggerBox.PlayerDetected` (`|GetArrayItem` _outactors (`self.TriggerBoxIndex`)) (delegate `PlayerTriggeredZone`))
    (else
      (bind _outactors_2 (`GameplayStatics.GetAllActorsOfClass` "/Game/Blueprints/GateCrank.GateCrank_C"))
      (add `/Game/Blueprints/GateCrank.GateOpened` (`|GetArrayItem` _outactors_2 (`self.GateCrankIndex`)) (delegate `OnFirstGateOpened`)))))

(event `PlayerTriggeredZone`
  (`ActorComponent.SetActive` (`self.FmodEvent`) true false :!label _label))

(event `OnFirstGateOpened`
  (goto _label))

(fn `UserConstructionScript`)