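; Gate Blueprint whose door slides between closed and open positions as crank input arrives.
; The UpdateCrank1 event adds a scaled-down input to a running Progress value.
; It then sets the door's world location by linearly interpolating between ClosedLocation and OpenLocation markers using that Progress, which is never clamped in this Blueprint.
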(event `/Game/Blueprints/GeneralInterface.UpdateCrank1`
  (params (Input :type "Float (single-precision)"))
  (`self.UpdateProgress` Input)
  (`self.Lerp between open and closed`))

(fn `Lerp between open and closed`
  (`SceneComponent.K2_SetWorldLocation` (`self.Door`) (`KismetMathLibrary.VLerp` (`SceneComponent.K2_GetComponentLocation` (`self.ClosedLocation`)) (`SceneComponent.K2_GetComponentLocation` (`self.OpenLocation`)) (`self.Progress`)) false false))

(fn `UpdateProgress`
  (params (A :type "Float (double-precision)"))
  (set `self.Progress` (+ (/ A 10.0) (`self.Progress`))))

(fn `UserConstructionScript`)